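; BP_CameraPawn is a player-controlled camera pawn that moves along its forward and right axes and zooms through a spring arm.
; BeginPlay registers the default Enhanced Input mapping context for the first player.
; Move input feeds a custom event that offsets actor location directly, without sweep or a movement component, scaled by speed and delta time.
; Zoom input adjusts arm length within clamped limits and prints it on screen for debugging.
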(event Custom|AddMovementInputCustom
  (params (WorldDirection :type Vector) (ScaleValue :type Float%20%28double-precision%29))
  (Transformation|SetActorLocation (+ (* WorldDirection ScaleValue (Variables|Default|GetMovementSpeed) (Utilities|Time|GetWorldDeltaSeconds)) (Transformation|GetActorLocation)) false false))

(event Input|EnhancedActionEvents|EnhancedInputActionIA_Move
  (params (ActionValue :type Vector%202D%20Structure) (ElapsedSeconds :type Float%20%28double-precision%29) (TriggeredSeconds :type Float%20%28double-precision%29) (InputAction :type Input%20Action%20Object%20Reference :default "/Game/Borealis/Input/IA_Move.IA_Move"))
  (CallFunction|AddMovementInputCustom (Transformation|GetActorRightVector) (.x ActionValue))
  (CallFunction|AddMovementInputCustom (Transformation|GetActorForwardVector) (.y ActionValue)))

(event Input|EnhancedActionEvents|EnhancedInputActionIA_Zoom
  (params (ActionValue :type Float%20%28double-precision%29) (ElapsedSeconds :type Float%20%28double-precision%29) (TriggeredSeconds :type Float%20%28double-precision%29) (InputAction :type Input%20Action%20Object%20Reference :default "/Game/Borealis/Input/IA_Zoom.IA_Zoom"))
  (bind _springarm (Variables|Default|GetSpringArm))
  (bind _output_get (Variables|/Script/Engine.SpringArmComponent|SetTargetArmLength _springarm (Math|Float|Clamp(Float) (+ (* ActionValue (Variables|Default|GetZoomSpeed) (Utilities|Time|GetWorldDeltaSeconds)) (Variables|/Script/Engine.SpringArmComponent|GetTargetArmLength _springarm)) 3e+02 6e+02)))
  (Development|PrintString (Utilities|String|Append "Target Arm Length: " (Utilities|String|ToString(Float) _output_get)) true false "(R=0.000000,G=0.660000,B=1.000000,A=1.000000)" 2.0 "TargetArmLength"))

(event EventBeginPlay
  (Input|AddMappingContext (PlayerController|LocalPlayerSubsystems|GetEnhancedInputLocalPlayerSubsystem (Game|GetPlayerController 0)) "/Game/Borealis/Input/IMC_Default.IMC_Default" 0 "(bIgnoreAllPressedKeysUntilRelease=True,bForceImmediately=False,bNotifyUserSettings=False)"))

(fn ConstructionScript)