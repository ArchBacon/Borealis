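; Player controller for Borealis that shows the mouse cursor and holds hex-grid coordinate math.
; A debug left-click traces under the cursor on the Visibility channel and prints the world impact point.
; PixelToHex converts X/Y to fractional cube coordinates with a fixed hex size, then CubeRound snaps them, recomputing the axis with the largest rounding error.
; The click handler does not call the hex conversion.
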(event EventBeginPlay
  (Variables|/Script/Engine.PlayerController|SetbShowMouseCursor (Game|GetPlayerController 0) true))

(event Input|MouseEvents|DebugKeyLeftMouseButton
  (params (Key :type Key%20Structure :default "None") (ActionValue :type Input%20Action%20Value%20Structure))
  (:Pressed
    (Development|PrintString (Utilities|String|ToString(Vector) (.ImpactPoint (Collision|BreakHitResult (.HitResult (Game|Player|GetHitResultUnderCursorbyChannel (Game|GetPlayerController 0) "TraceTypeQuery1" true))))))
    (Development|PrintString "Hello" true false "(R=0.000000,G=0.660000,B=1.000000,A=1.000000)" 1e+01)))

(fn ConstructionScript)

(fn PixeltoHex
  (params (X :type Float%20%28double-precision%29) (Y :type Float%20%28double-precision%29))
  (LocalVariables|SetQ (|((((sqrt(3))/3)*X)-(((1/3)*Y)/Size)) X Y 5e+01))
  (LocalVariables|SetR (|(((2/3)*Y)/Size) Y 5e+01))
  (return (CallFunction|CubeRound (Math|Vector|MakeVector (LocalVariables|GetQ) (LocalVariables|GetR) (- (* (LocalVariables|GetQ) -1.0) (LocalVariables|GetR))))))

(fn CubeRound
  (params (Frac :type Vector))
  (|SetQ (.x Frac))
  (|SetR (.y Frac))
  (|SetS (.z Frac))
  (Utilities|FlowControl|Sequence
    (:then_0
      (if (and (> (LocalVariables|GetQDiff) (LocalVariables|GetRDiff)) (> (LocalVariables|GetQDiff) (LocalVariables|GetSDiff)))
        (LocalVariables|SetQ (- (* (LocalVariables|GetR) -1) (LocalVariables|GetS)))
        (elif (> (LocalVariables|GetRDiff) (LocalVariables|GetSDiff))
          (LocalVariables|SetR (- (* (LocalVariables|GetQ) -1) (LocalVariables|GetS)))
          (else
            (LocalVariables|SetS (- (* (LocalVariables|GetQ) -1) (LocalVariables|GetR)))))))
    (:then_1
      (return (Utilities|Struct|MakeIntVector (LocalVariables|GetQ) (LocalVariables|GetR) (LocalVariables|GetS))))))